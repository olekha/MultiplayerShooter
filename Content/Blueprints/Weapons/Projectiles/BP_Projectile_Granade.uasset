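; Grenade projectile that is thrown as a spinning physics body and explodes after a delay.
; Activate launches the box with a forward impulse and random spin, while the server runs the fuse timer from BeginPlay.
; Explode applies full radial damage and destroys the actor, and remote clients spawn the explosion effect on Destroyed.
; GetPlayersToIgnore gathers nearby characters the game mode protects from damage, but Explode does not use it.
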(event Custom|Activate
  (bind _box (Variables|Default|GetBox))
  (Physics|SetSimulatePhysics _box true)
  (Physics|AddImpulse _box (* (Transformation|GetActorForwardVector) (Variables|Default|GetThrowPower)) "None" false)
  (Class|PrimitiveComponent|AddAngularImpulseinDegrees _box (Math|Vector|MakeVector (Math|Random|RandomFloatinRange 0.0 3.6e+02) (Math|Random|RandomFloatinRange 0.0 3.6e+02) (Math|Random|RandomFloatinRange 0.0 3.6e+02)) "None" false))

(event EventBeginPlay
  (|CallParentFunction)
  (Networking|SwitchHasAuthority
    (:Authority
      (Utilities|Time|SetTimerbyFunctionName 0 "Explode" (Variables|Default|GetExplosionDelay)))))

(event EventDestroyed
  (|CallParentFunction)
  (Networking|SwitchHasAuthority
    (:Remote
      (Effects|SpawnEmitteratLocation "/Game/Assets/Particles/P_Explosion.P_Explosion" (Transformation|GetActorLocation)))))

(fn ConstructionScript
  (|CallParentFunction))

(fn Explode
  (Game|Damage|ApplyRadialDamage (Variables|Default|GetDamage) (Transformation|GetActorLocation) (Variables|Default|GetExplosionRadius) 0 0 self (Game|GetInstigatorController) true "ECC_WorldStatic")
  (Actor|DestroyActor))

(fn GetPlayerstoIgnore
  (bind _returnvalue (Transformation|GetActorLocation))
  (bind _outhits (Collision|MultiSphereTraceForObjects _returnvalue _returnvalue (Variables|Default|GetExplosionRadius) (Utilities|Array|MakeArray "ObjectTypeQuery3") false 0 "None"))
  (for _array_element _outhits
    (bind _asbp_shooter_character (Utilities|Casting|CastToBP_ShooterCharacter (.HitActor (Collision|BreakHitResult _array_element))))
    (if (not (Default|ShouldDamagePlayer (CallFunction|GetSGameMode) (CallFunction|GetCharacterSController _asbp_shooter_character) (.AsBP%20Shooter%20Controller (Utilities|Casting|CastToBP_ShooterController (Game|GetInstigatorController)))))
      (Utilities|Array|Add (LocalVariables|GetPlayers) _asbp_shooter_character)))
  (return (LocalVariables|GetPlayers)))