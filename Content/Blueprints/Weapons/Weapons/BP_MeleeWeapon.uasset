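; Melee weapon Blueprint that deals point damage to what it hits in front of the shooter character, optionally spending stamina per use.
; Use is gated by the parent checks and the owner health component's stamina; a sphere trace from the camera along the owner's forward vector finds the hit.
; Selecting attaches it to the owner's mesh weapon socket, while deselecting hides it on the owner.
; Debug capsule traces and messages accompany attacks and selection changes.
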(event Custom|DebugDrawServerTrace
  (params (LineStart :type Vector) (LineEnd :type Vector) (Hit :type Vector))
  (Class|KismetSystemLibrary|CapsuleTraceSinglebyProfile LineStart LineEnd (Variables|MeleeWeaponSettings|GetWeaponUseRange) 1e+01 "None" false 0 "ForDuration" true))

(event EventBeginPlay
  (if (Variables|MeleeWeaponSettings|GetUseStamina)
    (Utilities|IsValid (Variables|Default|GetOwnerHealthComponent)
      (:Is%20Not%20Valid
        (Variables|MeleeWeaponSettings|SetUseStamina false)))))

(event Collision|EventActorBeginOverlap
  (params (OtherActor :type Actor%20Object%20Reference)))

(event EventTick
  (params (DeltaSeconds :type Float%20%28single-precision%29)))

(fn ConstructionScript
  (|CallParentFunction)
  (Variables|MeleeWeaponSettings|SetStaminaToReduce (Math|Float|Max(Float) (Variables|MeleeWeaponSettings|GetStaminaToReduce) 0.1))
  (Variables|MeleeWeaponSettings|SetWeaponUseRange (Math|Float|Max(Float) (Variables|MeleeWeaponSettings|GetWeaponUseRange) 1.0)))

(fn GetHitTrace
  (bind _asbp_shooter_character (Utilities|Casting|CastToBP_ShooterCharacter (Game|GetInstigator))
    (:then
      (bind _outhit (Collision|SphereTraceForObjects (Transformation|GetWorldLocation (Variables|/Game/Blueprints/Player/BP_ShooterCharacter.BP_ShooterCharacter_C|GetCamera _asbp_shooter_character)) (+ (Transformation|GetWorldLocation (Variables|/Game/Blueprints/Player/BP_ShooterCharacter.BP_ShooterCharacter_C|GetCamera _asbp_shooter_character)) (* (Transformation|GetActorForwardVector (Components|GetOwner)) (Variables|MeleeWeaponSettings|GetWeaponUseRange))) (Variables|MeleeWeaponSettings|GetWeaponUseRange) (Utilities|Array|MakeArray "ObjectTypeQuery1" "ObjectTypeQuery2" "ObjectTypeQuery3") false (Utilities|Array|MakeArray (Game|GetInstigator)) "None"))
      (CallFunction|DebugDrawServerTrace (.TraceStart (Collision|BreakHitResult _outhit)) (.TraceEnd (Collision|BreakHitResult _outhit)) (.Location (Collision|BreakHitResult _outhit)))
      (return _outhit))
    (:CastFailed
      (return ""))))

(fn StartUse
  (bind _isused (|CallParentFunction))
  (if _isused
    (Utilities|FlowControl|Sequence
      (:then_0
        (if (Variables|MeleeWeaponSettings|GetUseStamina)
          (Default|UseStamina (Variables|Default|GetOwnerHealthComponent) (Variables|MeleeWeaponSettings|GetStaminaToReduce))))
      (:then_1
        (bind _outhit (CallFunction|GetHitTrace))
        (Game|Damage|ApplyPointDamage (.HitActor (Collision|BreakHitResult _outhit)) (Variables|Default|GetDamageValue) (Math|Vector|GetUnitDirection(Vector) (.TraceEnd (Collision|BreakHitResult _outhit)) (.TraceStart (Collision|BreakHitResult _outhit))) _outhit (Game|GetInstigatorController) self)))
    (else
      (return false))))

(fn IsAbletoUse
  (bind _isable_ (|CallParentFunction))
  (if (Variables|MeleeWeaponSettings|GetUseStamina)
    (return (and (>= (- (.Stamina (Default|GetStamina (Variables|Default|GetOwnerHealthComponent))) (Variables|MeleeWeaponSettings|GetStaminaToReduce)) 0.0) _isable_))
    (else
      (return _isable_))))

(fn Select
  (params (IsSelect :type Boolean))
  (bind _succes (|CallParentFunction IsSelect))
  (if _succes
    (if IsSelect
      (Transformation|AttachComponentToComponent (Default|GetVisibleMesh (Variables|Default|GetWeaponOwner)) "Skt_Weapon" "SnapToTarget" "SnapToTarget" "SnapToTarget" true)
      (Rendering|SetActorHiddenInGame false)
      (|Debug_1)
      (return false)
      (else
        (Rendering|SetActorHiddenInGame true)
        (Transformation|AttachActorToActor (Variables|Default|GetWeaponOwner) "None" "SnapToTarget" "SnapToTarget" "KeepRelative" true)
        (|Debug_2)
        (return false)))))