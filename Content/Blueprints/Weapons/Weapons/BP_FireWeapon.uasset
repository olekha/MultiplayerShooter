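; Firearm weapon that adds ammo, reloading and firing to its parent weapon's select and use logic.
; Each shot spends a round, then spawns a BulletsType projectile or, without one, line-traces from the camera along owner forward for point damage.
; RepNotifies drive server-side reloading: an empty clip starts a timer, whose completion refills from reserve, while deselecting cancels it.
; Selection socket-attaches and shows the weapon; debug text and trace drawing remain active.
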(event Custom|DebugDrawServerTrace
  (params (LineStart :type Vector) (LineEnd :type Vector) (Hit :type Vector))
  (Rendering|Debug|DrawDebugLine LineStart LineEnd "(R=1.000000,G=0.000000,B=0.004948,A=1.000000)" 5.0 2.0)
  (Rendering|Debug|DrawDebugSphere Hit 4e+01 8 "(R=0.965966,G=1.000000,B=0.000000,A=1.000000)" 5.0 2.0))

(event Custom|ServerReloadFinished
  (Variables|Default|SetIsReloading false))

(event Custom|DebubShowAmmo
  (Rendering|Components|TextRender|SetText (Variables|Default|GetAmmo) (Utilities|Text|ToText(String) (Utilities|String|SelectString "RELOADING" (Utilities|String|Append (Utilities|String|ToString(Integer) (Variables|FireWeaponSettings|GetCurrentAmmo)) "  /  " (Utilities|String|ToString(Integer) (Variables|FireWeaponSettings|GetTotalAmmo)) (Utilities|String|SelectString " - R " "" (Variables|Default|GetIsRateDelay))) (Variables|Default|GetIsReloading)))))

(event EventTick
  (params (DeltaSeconds :type Float%20%28single-precision%29))
  (CallFunction|DebubShowAmmo)
  (Networking|SwitchHasAuthority
    (:Authority
      (Utilities|IsValid (Components|GetOwner)
        (:Is%20Valid
          (Utilities|PrintMessage (Utilities|String|ToString(Float) (Utilities|Time|GetTimerRemainingTimebyHandle (Variables|Default|GetReloadTimer))) false 0 1.0))))))

(fn ConstructionScript
  (|CallParentFunction)
  (Variables|FireWeaponSettings|SetReloadTime (Math|Float|Max(Float) (Variables|FireWeaponSettings|GetReloadTime) 0.1))
  (Variables|FireWeaponSettings|SetCurrentAmmo (Math|Integer|Clamp(Integer) (Variables|FireWeaponSettings|GetCurrentAmmo) 0 (Variables|FireWeaponSettings|GetClipCapacity)))
  (Variables|FireWeaponSettings|SetClipCapacity (Math|Integer|Max(Integer) (Variables|FireWeaponSettings|GetClipCapacity) 1))
  (Variables|FireWeaponSettings|SetTotalAmmo (Math|Integer|Max(Integer) (Variables|FireWeaponSettings|GetTotalAmmo))))

(fn GetFireTrace
  (bind _bp_shooter_character (Utilities|GetInstigatorMSCharacter)
    (:succes
      (bind _outhit (Collision|LineTraceForObjects (Transformation|GetWorldLocation (Variables|/Game/Blueprints/Player/BP_ShooterCharacter.BP_ShooterCharacter_C|GetCamera _bp_shooter_character)) (+ (Transformation|GetWorldLocation (Variables|/Game/Blueprints/Player/BP_ShooterCharacter.BP_ShooterCharacter_C|GetCamera _bp_shooter_character)) (* (Transformation|GetActorForwardVector (Components|GetOwner)) 1e+04)) (Utilities|Array|MakeArray "ObjectTypeQuery1" "ObjectTypeQuery2" "ObjectTypeQuery3") false (Utilities|Array|MakeArray (Game|GetInstigator)) "None"))
      (CallFunction|DebugDrawServerTrace (.TraceStart (Collision|BreakHitResult _outhit)) (.TraceEnd (Collision|BreakHitResult _outhit)) (.Location (Collision|BreakHitResult _outhit)))
      (return _outhit))
    (:Failed
      (return ""))))

(fn OnRepIsReloading
  (bind _clipcapacity (Variables|FireWeaponSettings|GetClipCapacity))
  (Networking|SwitchHasAuthority
    (:Authority
      (if (Variables|Default|GetIsReloading)
        (bind _returnvalue (Utilities|Time|SetTimerbyFunctionName 0 "ReloadFinished" (Variables|FireWeaponSettings|GetReloadTime)))
        (Variables|Default|SetReloadTimer _returnvalue)
        (elif (== (Utilities|Time|GetTimerRemainingTimebyHandle (Variables|Default|GetReloadTimer)) 0.0)
          (bind _output_get (LocalVariables|SetAmmoIncoming (Math|Integer|Min(Integer) (Math|Integer|SelectInt _clipcapacity (Variables|FireWeaponSettings|GetTotalAmmo) (>= (Variables|FireWeaponSettings|GetTotalAmmo) _clipcapacity)) (- (Variables|FireWeaponSettings|GetClipCapacity) (Variables|FireWeaponSettings|GetCurrentAmmo)))))
          (Variables|FireWeaponSettings|SetCurrentAmmo (+ _output_get (Variables|FireWeaponSettings|GetCurrentAmmo)))
          (Variables|FireWeaponSettings|SetTotalAmmo (- (Variables|FireWeaponSettings|GetTotalAmmo) (LocalVariables|GetAmmoIncoming)))
          (else
            (Utilities|Time|ClearandInvalidateTimerbyHandle (Variables|Default|GetReloadTimer))))))))

(fn ReloadFinished
  (CallFunction|ServerReloadFinished))

(fn InitiateReload
  (if (CallFunction|IsAbletoReload)
    (Variables|Default|SetIsReloading true)))

(fn IsAbletoReload
  (return (Math|Boolean|ANDBoolean (!= (Variables|FireWeaponSettings|GetTotalAmmo) 0) (!= (Variables|FireWeaponSettings|GetCurrentAmmo) (Variables|FireWeaponSettings|GetClipCapacity)) (not (Variables|Default|GetIsReloading)))))

(fn SpawnProjectile
  (bind _returnvalue (Components|GetOwner))
  (bind _returnvalue_2 (Transformation|GetActorForwardVector _returnvalue))
  (Networking|SwitchHasAuthority
    (:Authority
      (bind _bp_shooter_character (Utilities|GetInstigatorMSCharacter)
        (:succes
          (Game|SpawnActorfromClass (Variables|FireWeaponSettings|GetBulletsType) (Math|Transform|MakeTransform (+ (Transformation|GetWorldLocation (Variables|/Game/Blueprints/Player/BP_ShooterCharacter.BP_ShooterCharacter_C|GetCamera _bp_shooter_character)) (* _returnvalue_2 1e+02)) (Math|Conversions|RotationFromXVector _returnvalue_2)) "AlwaysSpawn" self (Variables|Default|GetDamageValue) (Game|GetInstigator)))))))

(fn OnRepCurrentAmmo
  (Networking|SwitchHasAuthority
    (:Authority
      (if (== (Variables|FireWeaponSettings|GetCurrentAmmo) 0)
        (CallFunction|InitiateReload)))))

(fn Select
  (params (IsSelect :type Boolean))
  (bind _succes (|CallParentFunction IsSelect))
  (if _succes
    (if IsSelect
      (Transformation|AttachComponentToComponent (Default|GetVisibleMesh (Variables|Default|GetWeaponOwner)) "Skt_Weapon" "SnapToTarget" "SnapToTarget" "SnapToTarget" true)
      (Rendering|SetActorHiddenInGame false)
      (Utilities|PrintMessage (Utilities|String|Append "Selected " (Utilities|GetDisplayName self) " by : ") true (Variables|Default|GetWeaponOwner) 15.0)
      (return true)
      (else
        (Rendering|SetActorHiddenInGame true)
        (Transformation|AttachActorToActor (Variables|Default|GetWeaponOwner) "None" "SnapToTarget" "SnapToTarget" "KeepRelative" true)
        (CallFunction|ReloadFinished)
        (Utilities|PrintMessage (Utilities|String|Append "Deselected " (Utilities|GetDisplayName self) " by : ") true (Variables|Default|GetWeaponOwner) 15.0)
        (return true)))))

(fn IsAbletoUse
  (return (Math|Boolean|ANDBoolean (|CallParentFunction) (not (Variables|Default|GetIsReloading)) (> (Variables|FireWeaponSettings|GetCurrentAmmo) 0))))

(fn StartUse
  (bind _isused (|CallParentFunction))
  (if _isused
    (Variables|FireWeaponSettings|SetCurrentAmmo (- (Variables|FireWeaponSettings|GetCurrentAmmo) 1))
    (if (Utilities|IsValidClass (Variables|FireWeaponSettings|GetBulletsType))
      (CallFunction|SpawnProjectile)
      (return true)
      (else
        (bind _outhit (CallFunction|GetFireTrace))
        (Game|Damage|ApplyPointDamage (.HitActor (Collision|BreakHitResult _outhit)) (Variables|Default|GetDamageValue) (Math|Vector|GetUnitDirection(Vector) (.TraceEnd (Collision|BreakHitResult _outhit)) (.TraceStart (Collision|BreakHitResult _outhit))) _outhit (Game|GetInstigatorController) self)
        (return true)))
    (elif (== (Variables|FireWeaponSettings|GetCurrentAmmo) 0)
      (CallFunction|InitiateReload)
      (return false))))