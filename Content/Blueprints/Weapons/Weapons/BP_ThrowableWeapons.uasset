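; Throwable weapon Blueprint for shooter characters, with a limited count that gates use.
; StartUse decrements the count and has the authority spawn a damage-carrying projectile in front of the camera, held attached to it with collision off.
; StopUse releases the projectile, re-enables collision and launches it at initial speed plus the thrower's velocity.
; Select shows the weapon on the hand socket or hides it on the owner.
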(event EventBeginPlay)

(event Collision|EventActorBeginOverlap
  (params (OtherActor :type Actor%20Object%20Reference)))

(event EventTick
  (params (DeltaSeconds :type Float%20%28single-precision%29)))

(fn ConstructionScript
  (|CallParentFunction))

(fn SpawnThrowable
  (bind _returnvalue (Components|GetOwner))
  (bind _returnvalue_2 (Transformation|GetActorForwardVector _returnvalue))
  (Networking|SwitchHasAuthority
    (:Authority
      (bind _asbp_shooter_character (Utilities|Casting|CastToBP_ShooterCharacter (Game|GetInstigator)))
      (bind _returnvalue_3 (Game|SpawnActorfromClass (Variables|WeaponSettings|ThrowableSettings|GetThrowableType) (Math|Transform|MakeTransform (+ (Transformation|GetWorldLocation (Variables|/Game/Blueprints/Player/BP_ShooterCharacter.BP_ShooterCharacter_C|GetCamera _asbp_shooter_character)) (* _returnvalue_2 3e+01)) (Math|Conversions|RotationFromXVector _returnvalue_2)) "AlwaysSpawn" self (Variables|Default|GetDamageValue) (Game|GetInstigator)))
      (bind _output_get (Variables|Default|SetCurrentProjectile _returnvalue_3))
      (return _output_get))))

(fn StartUse
  (bind _isused (|CallParentFunction))
  (if _isused
    (Variables|WeaponSettings|ThrowableSettings|SetCurrentAmount (- (Variables|WeaponSettings|ThrowableSettings|GetCurrentAmount) 1))
    (bind _newprojectile (CallFunction|SpawnThrowable))
    (Collision|SetActorEnableCollision _newprojectile false)
    (Transformation|AttachComponentToComponent _newprojectile (Variables|/Game/Blueprints/Player/BP_ShooterCharacter.BP_ShooterCharacter_C|GetCamera (.AsBP%20Shooter%20Character (Utilities|Casting|CastToBP_ShooterCharacter (Game|GetInstigator)))) "None" "KeepWorld" "KeepWorld" "KeepRelative" true)
    (return true)
    (else
      (return false))))

(fn Select
  (params (IsSelect :type Boolean))
  (bind _succes (|CallParentFunction IsSelect))
  (if _succes
    (if IsSelect
      (Transformation|AttachComponentToComponent (Default|GetVisibleMesh (Variables|Default|GetWeaponOwner)) "Skt_Weapon" "SnapToTarget" "SnapToTarget" "SnapToTarget" true)
      (Rendering|SetActorHiddenInGame false)
      (|Debug_1_2)
      (return true)
      (else
        (Rendering|SetActorHiddenInGame true)
        (Transformation|AttachActorToActor (Variables|Default|GetWeaponOwner) "None" "SnapToTarget" "SnapToTarget" "KeepRelative" true)
        (|Debug_2_2)
        (return true)))))

(fn StopUse
  (bind _isstopped (|CallParentFunction))
  (if _isstopped
    (bind _currentprojectile (Variables|Default|GetCurrentProjectile)
      (:then
        (Transformation|DetachFromComponent (Variables|/Game/Blueprints/Weapons/Projectiles/BP_Projectile.BP_Projectile_C|GetBox _currentprojectile) "KeepWorld" "KeepWorld" "KeepRelative" false)
        (Variables|/Script/Engine.MovementComponent|SetVelocity (Variables|/Game/Blueprints/Weapons/Projectiles/BP_Projectile.BP_Projectile_C|GetProjectileMovement _currentprojectile) (+ (* (Transformation|GetActorForwardVector _currentprojectile) (Variables|/Script/Engine.ProjectileMovementComponent|GetInitialSpeed (Variables|/Game/Blueprints/Weapons/Projectiles/BP_Projectile.BP_Projectile_C|GetProjectileMovement _currentprojectile))) (Transformation|GetVelocity (Game|GetInstigator))))
        (Components|Activation|Activate (Variables|/Game/Blueprints/Weapons/Projectiles/BP_Projectile.BP_Projectile_C|GetProjectileMovement _currentprojectile) false)
        (Collision|SetActorEnableCollision (Variables|Default|GetCurrentProjectile) true)
        (return true))
      (:else
        _)))
  (return false))

(fn IsAbletoUse
  (return (and (|CallParentFunction) (> (Variables|WeaponSettings|ThrowableSettings|GetCurrentAmount) 0))))