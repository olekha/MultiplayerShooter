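; BP_Weapon is a weapon Blueprint that gates use by ammo count and use rate.
; UseWeapon succeeds only when ammo remains and the rate freeze is off, then sets the freeze and starts a one-shot timer of UseRate length.
; StopRateDelay and Stop both clear the freeze.
; UseWeapon checks CurrentAmmo but does not decrement it.
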(event Custom|StopRateDelay
  (Variables|Default|SetUseFreezeByRate false))

(fn ConstructionScript)

(fn UseWeapon
  (if (CallFunction|IsAbletoUseAmmo)
    (Utilities|Time|SetTimerbyEvent (EventDispatchers|CreateEvent :!event Custom|StopRateDelay) (Variables|Default|GetUseRate))
    (Variables|Default|SetUseFreezeByRate true)
    (return true)
    (else
      (return false))))

(fn IsAbletoUseAmmo
  (return (and (not (Variables|Default|GetUseFreezeByRate)) (> (Variables|Default|GetCurrentAmmo) 0))))

(fn Stop
  (Variables|Default|SetUseFreezeByRate false)
  (return true))