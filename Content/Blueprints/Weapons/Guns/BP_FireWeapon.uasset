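; Firearm weapon Blueprint handling firing, ammo and timed reloads.
; Without a valid BulletsType, a shot spends ammo and applies point damage via a line trace from the instigator's camera along the owner's forward vector.
; Firing on an empty clip triggers reload through the IsReloading RepNotify, where authority transfers reserve ammo immediately and starts the timer that unblocks ammo use.
; Debug drawing and prints show traces and ammo.
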(event Custom|DebugDrowServerTrace
  (params (LineStart :type Vector) (LineEnd :type Vector) (Hit :type Vector))
  (Rendering|Debug|DrawDebugLine LineStart LineEnd "(R=1.000000,G=0.000000,B=0.004948,A=1.000000)" 5.0 2.0)
  (Rendering|Debug|DrawDebugSphere Hit 4e+01 8 "(R=0.965966,G=1.000000,B=0.000000,A=1.000000)" 5.0 2.0))

(event EventTick
  (params (DeltaSeconds :type Float%20%28single-precision%29))
  (|CallParentFunction DeltaSeconds)
  (Networking|SwitchHasAuthority
    (:Authority
      (Development|PrintString (Utilities|String|Append (Utilities|String|ToString(Integer) (Variables|Default|GetCurrentAmmo)) " | " (Utilities|String|ToString(Integer) (Variables|Default|GetTotalAmmo))) true true "(R=0.000000,G=0.660000,B=1.000000,A=1.000000)" 0.1))))

(fn ConstructionScript
  (|CallParentFunction))

(fn GetFireTrace
  (bind _bp_shooter_character (Utilities|GetInstigatorMSCharacter)
    (:succes
      (bind _outhit (Collision|LineTraceForObjects (Transformation|GetWorldLocation (Variables|/Game/Blueprints/Player/BP_ShooterCharacter.BP_ShooterCharacter_C|GetCamera _bp_shooter_character)) (+ (Transformation|GetWorldLocation (Variables|/Game/Blueprints/Player/BP_ShooterCharacter.BP_ShooterCharacter_C|GetCamera _bp_shooter_character)) (* (Transformation|GetActorForwardVector (Components|GetOwner)) 1e+04)) (Utilities|Array|MakeArray "ObjectTypeQuery1" "ObjectTypeQuery2" "ObjectTypeQuery3") false (Utilities|Array|MakeArray (Game|GetInstigator)) "ForDuration"))
      (CallFunction|DebugDrowServerTrace (.TraceStart (Collision|BreakHitResult _outhit)) (.TraceEnd (Collision|BreakHitResult _outhit)) (.Location (Collision|BreakHitResult _outhit)))
      (return _outhit))))

(fn StartUseWeapon
  (bind _isused (|CallParentFunction))
  (if _isused
    (if (Utilities|IsValidClass (Variables|Default|GetBulletsType))
      (return true)
      (else
        (Math|Integer|DecrementInt (Variables|Default|GetCurrentAmmo)
          (:%20%20
            (bind _outhit (CallFunction|GetFireTrace))
            (Game|Damage|ApplyPointDamage (.HitActor (Collision|BreakHitResult _outhit)) (Variables|Default|GetDamageValue) (Math|Vector|GetUnitDirection(Vector) (.TraceEnd (Collision|BreakHitResult _outhit)) (.TraceStart (Collision|BreakHitResult _outhit))) _outhit (Game|GetInstigatorController) self)
            (return true)))))
    (elif (== (Variables|Default|GetCurrentAmmo) 0)
      (CallFunction|InitiateReload)
      (return false))))

(fn OnRepIsReloading
  (bind _clipcapacity (Variables|Default|GetClipCapacity))
  (Networking|SwitchHasAuthority
    (:Authority
      (if (Variables|Default|GetIsReloading)
        (Utilities|Time|SetTimerbyFunctionName 0 "ReloadFinished" (Variables|Default|GetReloadTime))
        (bind _output_get (LocalVariables|SetAmmoIncoming (Math|Integer|Min(Integer) (Math|Integer|SelectInt _clipcapacity (Variables|Default|GetTotalAmmo) (>= (Variables|Default|GetTotalAmmo) _clipcapacity)) (- (Variables|Default|GetClipCapacity) (Variables|Default|GetCurrentAmmo)))))
        (Variables|Default|SetCurrentAmmo (+ _output_get (Variables|Default|GetCurrentAmmo)))
        (Variables|Default|SetTotalAmmo (- (Variables|Default|GetTotalAmmo) (LocalVariables|GetAmmoIncoming)))
        (Development|PrintString " 
RELOAD 
" true true "(R=1.000000,G=0.000000,B=0.008001,A=1.000000)" (Variables|Default|GetReloadTime))))))

(fn ReloadFinished
  (Variables|Default|SetIsReloading false))

(fn IsAbletoUseAmmo
  (return (and (|CallParentFunction) (not (Variables|Default|GetIsReloading)))))

(fn InitiateReload
  (if (CallFunction|IsAbletoReload)
    (Variables|Default|SetIsReloading true)))

(fn IsAbletoReload
  (return (and (!= (Variables|Default|GetTotalAmmo) 0) (!= (Variables|Default|GetCurrentAmmo) (Variables|Default|GetClipCapacity)))))