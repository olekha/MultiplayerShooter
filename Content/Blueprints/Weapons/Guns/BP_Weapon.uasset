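; BP_Weapon is a gun Blueprint that handles firing state and rate limiting.
; StartUseWeapon succeeds only when no rate delay is active and ammo remains, then flags firing and starts a UseRate timer.
; When the timer calls StopRateDelay, auto-fire weapons still firing re-trigger StartUseWeapon; otherwise firing ends.
; It contains no shot logic or ammo consumption, only the state flags and checks.
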(fn ConstructionScript)

(fn StartUseWeapon
  (if (CallFunction|IsAbletoUseAmmo)
    (Utilities|Time|SetTimerbyFunctionName 0 "StopRateDelay" (Variables|Default|GetUseRate))
    (Variables|Default|SetIsRateDelay true)
    (Variables|Default|SetIsFire true)
    (return true)
    (else
      (Variables|Default|SetIsFire false)
      (return false))))

(fn IsAbletoUseAmmo
  (return (and (not (Variables|Default|GetIsRateDelay)) (> (Variables|Default|GetCurrentAmmo) 0))))

(fn StopUseWeapon
  (Variables|Default|SetIsFire false))

(fn StopRateDelay
  (Variables|Default|SetIsRateDelay false)
  (Utilities|FlowControl|Sequence
    (:then_0
      (if (and (Variables|Default|GetIsAutoFire) (Variables|Default|GetIsFire))
        (CallFunction|StartUseWeapon)
        (else
          (Variables|Default|SetIsFire false))))
    (:then_1
      (return))))