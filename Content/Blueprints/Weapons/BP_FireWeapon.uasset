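; Fire weapon Blueprint that performs a hitscan shot on top of a parent weapon class.
; When the parent UseWeapon succeeds, GetFireTrace runs a Visibility line trace from the instigator character's camera along the owner's forward vector, ignoring the instigator.
; The trace is drawn as a debug line and sphere, with no damage applied here.
; StopRateDelay calls UseWeapon again when IsAutoFire is set, giving automatic fire.
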(event Custom|DebugDrowServerTrace
  (params (LineStart :type Vector) (LineEnd :type Vector) (Hit :type Vector))
  (Rendering|Debug|DrawDebugLine LineStart LineEnd "(R=1.000000,G=0.000000,B=0.004948,A=1.000000)" 5.0 2.0)
  (Rendering|Debug|DrawDebugSphere Hit 4e+01 8 "(R=0.965966,G=1.000000,B=0.000000,A=1.000000)" 5.0 2.0))

(event EventBeginPlay
  (|CallParentFunction) ; This node is disabled and will not be called.\nDrag off pins to build functionality.
)

(event Collision|EventActorBeginOverlap
  (params (OtherActor :type Actor%20Object%20Reference))
  (|CallParentFunction OtherActor) ; This node is disabled and will not be called.\nDrag off pins to build functionality.
)

(event EventStopRateDelay
  (|CallParentFunction)
  (Utilities|FlowControl|Sequence
    (:then_0
      (if (Variables|Default|GetIsAutoFire)
        (CallFunction|UseWeapon)))))

(event EventTick
  (params (DeltaSeconds :type Float%20%28single-precision%29))
  (|CallParentFunction DeltaSeconds) ; This node is disabled and will not be called.\nDrag off pins to build functionality.
)

(fn ConstructionScript
  (|CallParentFunction))

(fn UseWeapon
  (bind _isused (|CallParentFunction))
  (if _isused
    (CallFunction|GetFireTrace)
    (return true)
    (else
      (return false))))

(fn GetFireTrace
  (bind _bp_shooter_character (Utilities|GetInstigatorMSCharacter)
    (:succes
      (bind _outhit (Collision|LineTraceByChannel (Transformation|GetWorldLocation (Variables|/Game/Blueprints/Player/BP_ShooterCharacter.BP_ShooterCharacter_C|GetCamera _bp_shooter_character)) (+ (Transformation|GetWorldLocation (Variables|/Game/Blueprints/Player/BP_ShooterCharacter.BP_ShooterCharacter_C|GetCamera _bp_shooter_character)) (* (Transformation|GetActorForwardVector (Components|GetOwner)) 1e+04)) "TraceTypeQuery1" false (Utilities|Array|MakeArray (Game|GetInstigator)) "None"))
      (CallFunction|DebugDrowServerTrace (.TraceStart (Collision|BreakHitResult _outhit)) (.TraceEnd (Collision|BreakHitResult _outhit)) (.Location (Collision|BreakHitResult _outhit)))
      (return _outhit))))