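; Shooter HUD that owns the player's main HUD, tab menu and spectator menu widgets.
; On BeginPlay it creates all three from class variables for the owning player and adds them to the viewport.
; Toggle functions call each widget's AddToScreen or RemoveFromScreen, showing it only when BP_BaseGameState's AllowHUD is true.
; ToggleWidgets sets all three visibilities in one call.
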(event EventBeginPlay
  (Utilities|FlowControl|Sequence
    (:then_0
      ;[1 1 1] Spawn Supported WIdgets
      (Utilities|FlowControl|Sequence
        (:then_0
          (bind _returnvalue (UserInterface|CreateWidget (Variables|Default|GetHUDWidgetClass) (Game|Player|GetOwningPlayerController)))
          (bind _output_get (Variables|Default|SetHUDReference _returnvalue))
          (UserInterface|Viewport|AddtoViewport _output_get 0))
        (:then_1
          (bind _returnvalue_2 (UserInterface|CreateWidget (Variables|Default|GetTabMenuWidgetClass) (Game|Player|GetOwningPlayerController)))
          (bind _output_get_2 (Variables|Default|SetTabMenuReference _returnvalue_2))
          (UserInterface|Viewport|AddtoViewport _output_get_2 0))
        (:then_2
          (bind _returnvalue_3 (UserInterface|CreateWidget (Variables|Default|GetSpectatorWidgetClass) (Game|Player|GetOwningPlayerController)))
          (bind _output_get_3 (Variables|Default|SetSpectateMenuReference _returnvalue_3))
          (UserInterface|Viewport|AddtoViewport _output_get_3 0))))))

(fn ConstructionScript)

(fn ToggleTabMenu
  (params (IsShow :type Boolean))
  (bind _asbp_base_game_state (Utilities|Casting|CastToBP_BaseGameState (Game|GetGameState)))
  (if (and IsShow (Variables|/Game/Blueprints/Game/GameStates/BP_BaseGameState.BP_BaseGameState_C|GetAllowHUD _asbp_base_game_state))
    (bind _tabmenureference (Variables|Default|GetTabMenuReference)
      (:then
        (if (UserInterface|Viewport|IsinViewport _tabmenureference)
          (Default|AddtoScreen _tabmenureference)))
      (:else))
    (else
      (bind _tabmenureference_2 (Variables|Default|GetTabMenuReference)
        (:then
          (Default|RemovefromScreen _tabmenureference_2))
        (:else)))))

(fn ToggleHUD
  (params (IsShow :type Boolean))
  (bind _asbp_base_game_state (Utilities|Casting|CastToBP_BaseGameState (Game|GetGameState)))
  (if (and IsShow (Variables|/Game/Blueprints/Game/GameStates/BP_BaseGameState.BP_BaseGameState_C|GetAllowHUD _asbp_base_game_state))
    (bind _hudreference (Variables|Default|GetHUDReference)
      (:then
        (if (UserInterface|Viewport|IsinViewport _hudreference)
          (Default|AddtoScreen _hudreference)))
      (:else))
    (else
      (bind _hudreference_2 (Variables|Default|GetHUDReference)
        (:then
          (Default|RemovefromScreen _hudreference_2))
        (:else)))))

(fn ToggleSpectateMenu
  (params (IsShow :type Boolean))
  (bind _asbp_base_game_state (Utilities|Casting|CastToBP_BaseGameState (Game|GetGameState)))
  (if (and IsShow (Variables|/Game/Blueprints/Game/GameStates/BP_BaseGameState.BP_BaseGameState_C|GetAllowHUD _asbp_base_game_state))
    (bind _spectatemenureference (Variables|Default|GetSpectateMenuReference)
      (:then
        (if (UserInterface|Viewport|IsinViewport _spectatemenureference)
          (Default|AddtoScreen _spectatemenureference)))
      (:else))
    (else
      (bind _spectatemenureference_2 (Variables|Default|GetSpectateMenuReference)
        (:then
          (Default|RemovefromScreen _spectatemenureference_2))
        (:else)))))

(fn ToggleWidgets
  (params (ShowHUD :type Boolean) (ShowTabMenu :type Boolean) (ShowSpectMenu :type Boolean))
  (Utilities|FlowControl|Sequence
    (:then_0
      (CallFunction|ToggleHUD ShowHUD))
    (:then_1
      (CallFunction|ToggleTabMenu ShowTabMenu))
    (:then_2
      (CallFunction|ToggleSpectateMenu ShowSpectMenu))))