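; Deathmatch game state that keeps separate Players and Spectators lists of shooter player states.
; InGameStateBehaviors sorts the PlayerArray into the two lists using each player state's spectator check, and GetPlayers returns either list.
; Add helpers reject duplicates, while remove helpers verify the player's current role first.
; BecamePlayer switches a player's role in either direction, updating the spectator flag on success or re-adding to the original list if the add fails.
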(event EventBeginPlay
  (|CallParentFunction) ; This node is disabled and will not be called.\nDrag off pins to build functionality.
)

(event EventTick
  (params (DeltaSeconds :type Float%20%28single-precision%29)))

(fn ConstructionScript
  (|CallParentFunction))

(fn InGameStateBehaviors
  (for _array_element (Variables|Default|GetPlayerArray)
    (if (Default|CheckIsSpectator (.AsBP%20Shooter%20Player%20State (Utilities|Casting|CastToBP_ShooterPlayerState _array_element)) false)
      (CallFunction|AddtoSpectators (.AsBP%20Shooter%20Player%20State (Utilities|Casting|CastToBP_ShooterPlayerState _array_element)))
      (else
        (CallFunction|AddtoPlayers (.AsBP%20Shooter%20Player%20State (Utilities|Casting|CastToBP_ShooterPlayerState _array_element))))))
  (return true))

(fn GetPlayers
  (params (IsSpectators :type Boolean))
  (return (select IsSpectators (Variables|GameStateSettings|GetSpectators) (Variables|GameStateSettings|GetPlayers))))

(fn RemovefromSpectators
  (params (Player :type BP%20Shooter%20Player%20State%20Object%20Reference))
  (if (Default|CheckIsSpectator Player false)
    (bind _returnvalue (Utilities|Array|RemoveItem (Variables|GameStateSettings|GetSpectators) Player))
    (return _returnvalue)
    (else
      (return false))))

(fn RemovefromPlayers
  (params (Player :type BP%20Shooter%20Player%20State%20Object%20Reference))
  (if (not (Default|CheckIsSpectator Player false))
    (bind _returnvalue (Utilities|Array|RemoveItem (Variables|GameStateSettings|GetPlayers) Player))
    (return _returnvalue)
    (else
      (return false))))

(fn AddtoSpectators
  (params (Player :type BP%20Shooter%20Player%20State%20Object%20Reference%20%28by%20ref%29))
  (if (== (Utilities|Array|FindItem (Variables|GameStateSettings|GetSpectators) Player) -1)
    (Utilities|Array|Add (Variables|GameStateSettings|GetSpectators) Player)
    (return true)
    (else
      (return false))))

(fn AddtoPlayers
  (params (Player :type BP%20Shooter%20Player%20State%20Object%20Reference%20%28by%20ref%29))
  (if (== (Utilities|Array|FindItem (Variables|GameStateSettings|GetPlayers) Player) -1)
    (Utilities|Array|Add (Variables|GameStateSettings|GetPlayers) Player)
    (return true)
    (else
      (return false))))

(fn BecamePlayer
  (params (IsSpectator :type Boolean) (Player :type BP%20Shooter%20Player%20State%20Object%20Reference))
  (if (Math|Boolean|NotEqual(Boolean) IsSpectator (Default|CheckIsSpectator Player false))
    (if IsSpectator
      (bind _success (CallFunction|RemovefromPlayers Player))
      (if _success
        (bind _success_2 (CallFunction|AddtoSpectators Player))
        (if _success_2
          (Default|SetIsSpectator Player true true)
          (else
            (CallFunction|AddtoPlayers Player))))
      (else
        (bind _success_3 (CallFunction|RemovefromSpectators Player))
        (if _success_3
          (bind _success_4 (CallFunction|AddtoPlayers Player))
          (if _success_4
            (Default|SetIsSpectator Player false true)
            (else
              (CallFunction|AddtoSpectators Player))))))))