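; BP_PostGameState is the game state for the post-game phase, carrying over the round time from the previous state.
; On BeginPlay, only the remote (non-authority) side sets the current round time, built from the previous state's minutes and seconds.
; An unconnected loop over PlayerArray would show the post-round menu on each valid controller's HUD, but it never runs.
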(event EventBeginPlay
  (Networking|SwitchHasAuthority
    (:Remote
      (CallFunction|SetCurrentRoundTime (Math|Timespan|MakeTimespan 0 0 (Variables|GameStateSettings|PostGameSettings|GetPreviousStateMinutes) (Variables|GameStateSettings|PostGameSettings|GetPreviousStateSeconds))))))

(fn ConstructionScript
  (|CallParentFunction))