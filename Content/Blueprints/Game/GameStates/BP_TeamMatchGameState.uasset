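; Game state for a two-team match that tracks Team A and Team B scores, their rosters and a spectator list.
; A death awards one point to the instigator's team when victim and instigator are on different teams.
; On authority during pre-game, the play-time tick sorts PlayerArray into rosters when the seconds value reaches 1.
; Helper functions handle roster lookups and team switches, re-adding players to their old team if joining the new one reports failure.
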(event EventBeginPlay
  (|CallParentFunction) ; This node is disabled and will not be called.\nDrag off pins to build functionality.
)

(event EventPlayerDiedEvent
  (params (DeadPlayer :type BP%20Shooter%20Controller%20Object%20Reference) (DeadPlayerCharacter :type BP%20Shooter%20Character%20Object%20Reference) (Instigator :type BP%20Shooter%20Controller%20Object%20Reference) (InstigatorCharacter :type BP%20Shooter%20Character%20Object%20Reference) (DeathCauser :type Actor%20Object%20Reference))
  (bind _playerstate (Variables|/Script/Engine.Controller|GetPlayerState Instigator))
  (bind _asbp_team_player_state (Utilities|Casting|CastToBP_TeamPlayerState _playerstate))
  (bind _team (Default|GetPlayerTeam _asbp_team_player_state))
  (|CallParentFunction DeadPlayer DeadPlayerCharacter Instigator InstigatorCharacter DeathCauser)
  (if (Utilities|Enum|NotEqual(Enum) (Default|GetPlayerTeam (.AsBP%20Team%20Player%20State (Utilities|Casting|CastToBP_TeamPlayerState (Variables|/Script/Engine.Controller|GetPlayerState DeadPlayer)))) _team)
    (CallFunction|AddPoints _team 1)))

(event EventPlayTimeTick
  (|CallParentFunction)
  (Networking|SwitchHasAuthority
    (:Authority
      (switch Utilities|FlowControl|Switch|SwitchonE_GameStateTypes (Variables|Default|GetCurrentType)
        (:NewEnumerator0
          (if (== (Math|Timespan|GetSeconds (CallFunction|GetCurrentTime)) 1)
            (for _array_element (Variables|Default|GetPlayerArray)
              (Utilities|Array|Add (Utilities|Select :Index (Default|GetPlayerTeam (.AsBP%20Team%20Player%20State (Utilities|Casting|CastToBP_TeamPlayerState _array_element))) :NewEnumerator0 (Variables|GameStateSettings|InGameSettings|TeamStateSettings|GetTeamAPlayers) :NewEnumerator1 (Variables|GameStateSettings|inGameSettings|TeamStateSettings|GetTeamBPlayers) :NewEnumerator3 (Variables|GameStateSettings|inGameSettings|TeamStateSettings|GetSpectators)) (.AsBP%20Team%20Player%20State (Utilities|Casting|CastToBP_TeamPlayerState _array_element))))))))))

(fn ConstructionScript
  (|CallParentFunction))

(fn GetTeamPoints
  (params (Team :type E_Teams%20Enum :default "NewEnumerator0"))
  (switch Utilities|FlowControl|Switch|SwitchonE_Teams Team
    (:NewEnumerator0
      (return (.points (Variables|GameStateSettings|inGameSettings|TeamStateSettings|GetTeamAPoints))))
    (:NewEnumerator1
      (return (.points (Variables|GameStateSettings|inGameSettings|TeamStateSettings|GetTeamBPoints))))
    (:NewEnumerator3
      (return -1))))

(fn AddPoints
  (params (Team :type E_Teams%20Enum :default "NewEnumerator0") (Points :type Integer))
  (switch Utilities|FlowControl|Switch|SwitchonE_Teams Team
    (:NewEnumerator0
      (Variables|GameStateSettings|inGameSettings|TeamStateSettings|SetTeamAPoints (Utilities|Struct|MakeST_Teams (.team (Variables|GameStateSettings|inGameSettings|TeamStateSettings|GetTeamAPoints)) (+ (.points (Variables|GameStateSettings|inGameSettings|TeamStateSettings|GetTeamAPoints)) Points))))
    (:NewEnumerator1
      (Variables|GameStateSettings|inGameSettings|TeamStateSettings|SetTeamBPoints (Utilities|Struct|MakeST_Teams (.team (Variables|GameStateSettings|inGameSettings|TeamStateSettings|GetTeamBPoints)) (+ Points (.points (Variables|GameStateSettings|inGameSettings|TeamStateSettings|GetTeamBPoints))))))))

(fn GetPlayers
  (params (Team :type E_Teams%20Enum :default "NewEnumerator0"))
  (switch Utilities|FlowControl|Switch|SwitchonE_Teams Team
    (:NewEnumerator0
      (return (Variables|GameStateSettings|InGameSettings|TeamStateSettings|GetTeamAPlayers)))
    (:NewEnumerator1
      (return (Variables|GameStateSettings|inGameSettings|TeamStateSettings|GetTeamBPlayers)))
    (:NewEnumerator3
      (return (Variables|GameStateSettings|inGameSettings|TeamStateSettings|GetSpectators)))))

(fn AddtoTeam
  (params (Player :type BP%20Team%20Player%20State%20Object%20Reference%20%28by%20ref%29) (NewTeam :type E_Teams%20Enum :default "NewEnumerator0"))
  (if (or (Utilities|Enum|NotEqual(Enum) (Default|GetPlayerTeam Player) NewTeam) (and (== (Default|GetPlayerTeam Player) NewTeam) (== (Utilities|Array|FindItem (CallFunction|GetPlayers (Default|GetPlayerTeam Player)) Player) -1)))
    (switch Utilities|FlowControl|Switch|SwitchonE_Teams NewTeam
      (:NewEnumerator0
        (Utilities|Array|Add (Variables|GameStateSettings|InGameSettings|TeamStateSettings|GetTeamAPlayers) Player)
        (return true))
      (:NewEnumerator1
        (Utilities|Array|Add (Variables|GameStateSettings|inGameSettings|TeamStateSettings|GetTeamBPlayers) Player)
        (return true))
      (:NewEnumerator3
        (Utilities|Array|Add (Variables|GameStateSettings|inGameSettings|TeamStateSettings|GetSpectators) Player)
        (return false)))
    (else
      (return false))))

(fn RemovefromTeam
  (params (Player :type BP%20Team%20Player%20State%20Object%20Reference%20%28by%20ref%29) (Team :type E_Teams%20Enum :default "NewEnumerator0"))
  (if (Utilities|Enum|Equal(Enum) (Default|GetPlayerTeam Player) Team)
    (switch Utilities|FlowControl|Switch|SwitchonE_Teams Team
      (:NewEnumerator0
        (bind _returnvalue (Utilities|Array|RemoveItem (Variables|GameStateSettings|InGameSettings|TeamStateSettings|GetTeamAPlayers) Player))
        (return _returnvalue))
      (:NewEnumerator1
        (bind _returnvalue_2 (Utilities|Array|RemoveItem (Variables|GameStateSettings|inGameSettings|TeamStateSettings|GetTeamBPlayers) Player))
        (return _returnvalue_2))
      (:NewEnumerator3
        (bind _returnvalue_3 (Utilities|Array|RemoveItem (Variables|GameStateSettings|inGameSettings|TeamStateSettings|GetSpectators) Player))
        (return _returnvalue_3)))
    (else
      (return false))))

(fn ChangePlayerTeam
  (params (Player :type BP%20Team%20Player%20State%20Object%20Reference) (NewTeam :type E_Teams%20Enum :default "NewEnumerator0"))
  (bind _team (Default|GetPlayerTeam Player))
  (if (Utilities|Enum|NotEqual(Enum) (Default|GetPlayerTeam Player) NewTeam)
    (bind _success (CallFunction|RemovefromTeam Player _team))
    (if _success
      (bind _success_2 (CallFunction|AddtoTeam Player NewTeam))
      (if _success_2
        (Default|SetTeam Player NewTeam)
        (else
          (CallFunction|AddtoTeam Player _team))))))

(fn GetOppositTeam
  (params (Player :type BP%20Team%20Player%20State%20Object%20Reference))
  (return (Utilities|Select :Index (Default|GetPlayerTeam Player) :NewEnumerator0 "NewEnumerator1" :NewEnumerator1 "NewEnumerator0" :NewEnumerator3 "NewEnumerator3")))