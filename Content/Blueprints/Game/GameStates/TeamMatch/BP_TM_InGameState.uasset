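; BP_TM_InGameState is the team match in-game state, which keeps score by awarding points to teams for kills.
; On a player death it runs the parent handler, then gives the instigator's team one point if the victim is on a different team.
; Points live in an array of team structs, written by using the team value as the index and read by searching for the team, returning -1 if absent.
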(event EventPlayerDiedEvent
  (params (DeadPlayer :type BP%20Shooter%20Controller%20Object%20Reference) (DeadPlayerCharacter :type BP%20Shooter%20Character%20Object%20Reference) (Instigator :type BP%20Shooter%20Controller%20Object%20Reference) (InstigatorCharacter :type BP%20Shooter%20Character%20Object%20Reference) (DeathCauser :type Actor%20Object%20Reference))
  (bind _playerstate (Variables|/Script/Engine.Controller|GetPlayerState Instigator))
  (bind _asbp_team_player_state (Utilities|Casting|CastToBP_TeamPlayerState _playerstate))
  (bind _team (Variables|/Game/Blueprints/Player/BP_TeamPlayerState.BP_TeamPlayerState_C|GetTeam _asbp_team_player_state))
  (|CallParentFunction DeadPlayer DeadPlayerCharacter Instigator InstigatorCharacter DeathCauser)
  (if (Utilities|Enum|NotEqual(Enum) (Variables|/Game/Blueprints/Player/BP_TeamPlayerState.BP_TeamPlayerState_C|GetTeam (.AsBP%20Team%20Player%20State (Utilities|Casting|CastToBP_TeamPlayerState (Variables|/Script/Engine.Controller|GetPlayerState DeadPlayer)))) _team)
    (CallFunction|AddPointstoTeam _team 1)))

(fn ConstructionScript
  (|CallParentFunction))

(fn GetTeamPoints
  (params (Team :type E_Teams%20Enum :default "NewEnumerator0"))
  (for _array_element (Variables|Default|GetTeamPoints)
    (if (Utilities|Enum|Equal(Enum) (.Team (Utilities|Struct|BreakST_Teams _array_element)) Team)
      (return (.Points (Utilities|Struct|BreakST_Teams _array_element)))))
  (return -1))

(fn AddPointstoTeam
  (params (Team :type E_Teams%20Enum :default "NewEnumerator0") (Points :type Integer))
  (bind _returnvalue (Math|Conversions|ToInteger(Byte) Team))
  (bind _teampoints (Variables|Default|GetTeamPoints))
  (bind _output (Utilities|Array|Get(acopy) _teampoints _returnvalue))
  (bind (_team _points) (Utilities|Struct|BreakST_Teams _output))
  (Utilities|Array|SetArrayElem (Variables|Default|GetTeamPoints) _returnvalue (Utilities|Struct|MakeST_Teams _team (+ _points Points))))