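; BP_PreGameState is the pre-game state, running a countdown before the game mode changes to another game state.
; It starts the game timer on BeginPlay, and on each authority play-time tick stores WaitTime minus current time as minutes and seconds.
; When the remainder equals zero, a one-shot Stopped flag guards the state change.
; GetTimeLeft rebuilds the remaining time from those stored values.
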(event EventBeginPlay
  (CallFunction|StartGameTimer))

(event EventPlayTimeTick
  (|CallParentFunction)
  (Networking|SwitchHasAuthority
    (:Authority
      (bind _output_get (Variables|Default|SetReversTimer (- (Variables|Default|GetWaitTime) (CallFunction|GetCurrentTime))))
      (Variables|Default|SetReversMinutes (.Minutes (Math|Timespan|BreakTimespan _output_get)))
      (Variables|Default|SetReversSeconds (.Seconds (Math|Timespan|BreakTimespan _output_get)))
      (if (and (== (Variables|Default|GetReversTimer) (Math|Timespan|MakeTimespan 0)) (not (Variables|Default|GetStopped)))
        (Variables|Default|SetStopped true)
        (Default|ChangeGameState (CallFunction|GetSGameMode) "NewEnumerator1")))))

(fn ConstructionScript
  (|CallParentFunction))

(fn GetTimeLeft
  (return (Math|Timespan|MakeTimespan 0 0 (Variables|Default|GetReversMinutes) (Variables|Default|GetReversSeconds))))