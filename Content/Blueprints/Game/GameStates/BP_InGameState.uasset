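; In-game GameState that keeps separate lists of active players and spectators for the match.
; On BeginPlay the server sorts every BP_ShooterPlayerState in PlayerArray into one list by its spectator flag.
; BecamePlayer moves a player between lists through guarded add and remove helpers, updating the flag on success and re-adding to the original list if the add fails.
; On Tick the server prints both counts as debug text.
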(event EventBeginPlay
  (|CallParentFunction)
  (Networking|SwitchHasAuthority
    (:Authority
      (for _array_element (Variables|Default|GetPlayerArray)
        (if (Default|CheckIsSpectator (.AsBP%20Shooter%20Player%20State (Utilities|Casting|CastToBP_ShooterPlayerState _array_element)) false)
          (CallFunction|AddtoSpectators (.AsBP%20Shooter%20Player%20State (Utilities|Casting|CastToBP_ShooterPlayerState _array_element)))
          (else
            (CallFunction|AddtoPlayers (.AsBP%20Shooter%20Player%20State (Utilities|Casting|CastToBP_ShooterPlayerState _array_element)))))))))

(event EventTick
  (params (DeltaSeconds :type Float%20%28single-precision%29))
  (Networking|SwitchHasAuthority
    (:Authority
      (Development|PrintString (Utilities|String|Append " Spect : " (Utilities|String|ToString(Integer) (Utilities|Array|Length (Variables|Default|GetSpectators))) " Plye : " (Utilities|String|ToString(Integer) (Utilities|Array|Length (Variables|Default|GetPlayers)))) true true "(R=0.000000,G=0.660000,B=1.000000,A=1.000000)" 0.0))))

(fn ConstructionScript
  (|CallParentFunction))

(fn GetPlayers
  (params (IsSpectators :type Boolean))
  (return (select IsSpectators (Variables|Default|GetSpectators) (Variables|Default|GetPlayers))))

(fn RemovefromSpectators
  (params (Player :type BP%20Shooter%20Player%20State%20Object%20Reference%20%28by%20ref%29))
  (if (Default|CheckIsSpectator Player false)
    (bind _returnvalue (Utilities|Array|RemoveItem (Variables|Default|GetSpectators) Player))
    (return _returnvalue)
    (else
      (return true))))

(fn RemovefromPlayers
  (params (Player :type BP%20Shooter%20Player%20State%20Object%20Reference%20%28by%20ref%29))
  (if (not (Default|CheckIsSpectator Player false))
    (bind _returnvalue (Utilities|Array|RemoveItem (Variables|Default|GetPlayers) Player))
    (return _returnvalue)
    (else
      (return true))))

(fn AddtoSpectators
  (params (Player :type BP%20Shooter%20Player%20State%20Object%20Reference%20%28by%20ref%29))
  (if (== (Utilities|Array|FindItem (Variables|Default|GetSpectators) Player) -1)
    (Utilities|Array|Add (Variables|Default|GetSpectators) Player)
    (return true)
    (else
      (return false))))

(fn AddtoPlayers
  (params (Player :type BP%20Shooter%20Player%20State%20Object%20Reference%20%28by%20ref%29))
  (if (== (Utilities|Array|FindItem (Variables|Default|GetPlayers) Player) -1)
    (Utilities|Array|Add (Variables|Default|GetPlayers) Player)
    (return true)
    (else
      (return false))))

(fn BecamePlayer
  (params (Player :type BP%20Shooter%20Player%20State%20Object%20Reference) (IsSpectator :type Boolean))
  (if (Math|Boolean|NotEqual(Boolean) IsSpectator (Default|CheckIsSpectator Player false))
    (if IsSpectator
      (bind _success (CallFunction|RemovefromPlayers Player))
      (if _success
        (bind _success_2 (CallFunction|AddtoSpectators Player))
        (if _success_2
          (Default|SetIsSpectator Player true true)
          (else
            (CallFunction|AddtoPlayers Player))))
      (else
        (bind _success_3 (CallFunction|RemovefromSpectators Player))
        (if _success_3
          (bind _success_4 (CallFunction|AddtoPlayers Player))
          (if _success_4
            (Default|SetIsSpectator Player false true)
            (else
              (CallFunction|AddtoSpectators Player))))))))