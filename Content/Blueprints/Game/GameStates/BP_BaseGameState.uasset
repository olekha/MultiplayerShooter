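; Base game state that keeps an elapsed-time clock for rounds.
; On the authority, BeginPlay binds to BP_BaseGameMode's RoundStarted and RoundEnded events to start and stop a looping one-second timer.
; Each tick adds a second to the RoundTime timespan and splits it into components that GetRoundTime returns.
; Stopping clears the timer but leaves the accumulated time intact.
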(event Custom|RoundStarted_Event_0
  (CallFunction|StartGameTimer))

(event Custom|RoundEnded_Event_0
  (params (REason :type E_RoundFinishReasons%20Enum :default "NewEnumerator0"))
  (CallFunction|StopGameTimer))

(event EventBeginPlay
  (Networking|SwitchHasAuthority
    (:Authority
      (bind _asbp_base_game_mode (Utilities|Casting|CastToBP_BaseGameMode (Game|GetGameMode)))
      (EventDispatchers|AssignRoundStarted _asbp_base_game_mode (delegate Custom|RoundStarted_Event_0))
      (EventDispatchers|AssignRoundEnded _asbp_base_game_mode (delegate Custom|RoundEnded_Event_0)))))

(fn ConstructionScript)

(fn StartGameTimer
  (bind _returnvalue (Utilities|Time|SetTimerbyFunctionName 0 "PlayTimeTick" 1.0 true))
  (Variables|Default|SetRoundTimerHandle _returnvalue))

(fn PlayTimeTick
  (bind _output_get (Variables|Default|SetRoundTime (+ (Variables|Default|GetRoundTime) (Math|Timespan|MakeTimespan 0 0 0 1))))
  (Variables|Default|SetHours (.Hours (Math|Timespan|BreakTimespan _output_get)))
  (Variables|Default|SetMinutes (.Minutes (Math|Timespan|BreakTimespan _output_get)))
  (Variables|Default|SetSeconds (.Seconds (Math|Timespan|BreakTimespan _output_get)))
  (Variables|Default|SetMilliSeconds (.Milliseconds (Math|Timespan|BreakTimespan _output_get))))

(fn StopGameTimer
  (Utilities|Time|ClearandInvalidateTimerbyHandle (Variables|Default|GetRoundTimerHandle)))

(fn GetRoundTime
  (return (Variables|Default|GetHours) (Variables|Default|GetMinutes) (Variables|Default|GetSeconds) (Variables|Default|GetMilliSeconds)))