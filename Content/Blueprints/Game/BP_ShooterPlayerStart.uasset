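; BP_ShooterPlayerStart is a player start that spawns a BP_ShooterCharacter at its transform and has the given player possess it.
; SpawnChracter stores the new pawn as CharacterInside, notifies BP_BaseGameMode through CallCharacterSpawned and returns the character.
; IsFree reports the start as available while CharacterInside is invalid, and the capsule's end-overlap event clears that reference when the spawned character leaves.
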(event OnComponentEndOverlap(CapsuleComponent)
  (params (OverlappedComponent :type Primitive%20Component%20Object%20Reference) (OtherActor :type Actor%20Object%20Reference) (OtherComp :type Primitive%20Component%20Object%20Reference) (OtherBodyIndex :type Integer))
  (if (== OtherActor (Variables|Default|GetCharacterInside))
    (Variables|Default|SetCharacterInside 0)))

(event EventBeginPlay)

(event EventTick
  (params (DeltaSeconds :type Float%20%28single-precision%29)))

(fn ConstructionScript)

(fn SpawnChracter
  (params (NewPlayer :type BP%20Shooter%20Controller%20Object%20Reference))
  (bind _output_get (LocalVariables|SetL_player NewPlayer))
  (bind _returnvalue (Game|SpawnActorfromClass "/Game/Blueprints/Player/BP_ShooterCharacter.BP_ShooterCharacter_C" (Transformation|GetActorTransform) "Undefined" _output_get 0))
  (bind _output_get_2 (Variables|Default|SetCharacterInside _returnvalue))
  (Pawn|Possess (LocalVariables|GetL_player) _output_get_2)
  (bind _asbp_base_game_mode (Utilities|Casting|CastToBP_BaseGameMode (Game|GetGameMode)))
  (Default|CallCharacterSpawned _asbp_base_game_mode (LocalVariables|GetL_player) (Variables|Default|GetCharacterInside))
  (return (Variables|Default|GetCharacterInside)))

(fn IsFree
  (return (not (Utilities|IsValid (Variables|Default|GetCharacterInside)))))