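; Deathmatch game mode that ends the round when a player reaches the kill limit.
; On each player death, after running parent logic, it checks the instigator's kill count if the kill-limit option is on.
; When the limit is met, it stores that player as winner in the deathmatch game state, waits briefly, then ends the round with character destruction and changes the game state.
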(event EventBeginPlay
  (|CallParentFunction) ; This node is disabled and will not be called.\nDrag off pins to build functionality.
)

(event EventTick
  (params (DeltaSeconds :type Float%20%28single-precision%29))
  (|CallParentFunction DeltaSeconds) ; This node is disabled and will not be called.\nDrag off pins to build functionality.
)

(event EventPlayerDiedEvent
  (params (DeadPlayer :type BP%20Shooter%20Controller%20Object%20Reference) (DeadPlayerCharacter :type BP%20Shooter%20Character%20Object%20Reference) (Instigator :type BP%20Shooter%20Controller%20Object%20Reference) (InstigatorCharacter :type BP%20Shooter%20Character%20Object%20Reference) (DeathCauser :type Actor%20Object%20Reference))
  (bind _splayerstate (CallFunction|GetControllerSPlayerState Instigator))
  (|CallParentFunction DeadPlayer DeadPlayerCharacter Instigator InstigatorCharacter DeathCauser)
  (if (Variables|GameModeSettings|Limits|GetIsLimitByKills)
    (if (>= (Variables|/Game/Blueprints/Player/BP_ShooterPlayerState.BP_ShooterPlayerState_C|GetKills _splayerstate) (Variables|GameModeSettings|Limits|GetKillLimit))
      (Variables|/Game/Blueprints/Game/GameStates/BP_DeathMatchGameState.BP_DeathMatchGameState_C|SetWinnerPlayer (CallFunction|GetDMGameState) _splayerstate)
      (Utilities|FlowControl|Delay 0.2)
      (CallFunction|EndRound "NewEnumerator1" true)
      (CallFunction|ChangeGameState "NewEnumerator2"))))

(fn ConstructionScript
  (|CallParentFunction))