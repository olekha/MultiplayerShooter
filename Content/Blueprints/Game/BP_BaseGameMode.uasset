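; Base game mode for a shooter that runs the round lifecycle, player spawning and spectating.
; After a short delay it spawns an in-game state actor, places players at shuffled free starts and optionally polls a time limit.
; Deaths optionally start a PlayerState respawn timer and always possess a spectator, following the killer if valid, otherwise free.
; Round end moves players to spectators and spawns a post-game state actor.
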(event Custom|PlayerDied_Event
  (params (DeadPlayer :type BP%20Shooter%20Controller%20Object%20Reference) (DeadPlayerCharacter :type BP%20Shooter%20Character%20Object%20Reference) (InstigatorPlayer :type BP%20Shooter%20Controller%20Object%20Reference) (DeathCauser :type Actor%20Object%20Reference))
  (Utilities|FlowControl|Sequence
    (:then_0
      (if (Variables|Respawn|GetIsAutoRespawn)
        (bind _asbp_shooter_player_state (Utilities|Casting|CastToBP_ShooterPlayerState (Variables|/Script/Engine.Controller|GetPlayerState DeadPlayer)))
        (Default|LaunchRespawnTimer _asbp_shooter_player_state (Variables|Respawn|GetRespawnTime))))
    (:then_1
      (CallFunction|SpawnSpectator DeadPlayer InstigatorPlayer))))

(event Custom|RoundEnded_Event
  (params (Reason :type E_RoundFinishReasons%20Enum :default "NewEnumerator0"))
  (Game|SpawnActorfromClass "/Game/Blueprints/Game/GameStates/BP_PostGameSstate.BP_PostGameSstate_C" (Math|Transform|MakeTransform "0, 0, 0") "AlwaysSpawn" 0 0))

(event EventBeginPlay
  (EventDispatchers|BindEventtoPlayerDied (EventDispatchers|CreateEvent :!event Custom|PlayerDied_Event))
  (EventDispatchers|BindEventtoRoundEnded (EventDispatchers|CreateEvent :!event Custom|RoundEnded_Event))
  (Utilities|FlowControl|Delay 3.0)
  (Game|SpawnActorfromClass "/Game/Blueprints/Game/GameStates/BP_InGameState.BP_InGameState_C" (Math|Transform|MakeTransform "0, 0, 0") "AlwaysSpawn" 0 0)
  (CallFunction|Start/EndRound true "NewEnumerator0")
  (if (Variables|Limits|GetIsLimitedByTime)
    (CallFunction|LaunchTimeChecker)))

(fn ConstructionScript)

(fn SpawnPlayer
  (params (Player :type BP%20Shooter%20Controller%20Object%20Reference))
  (bind _outactors (Actor|GetAllActorsOfClass "/Game/Blueprints/Game/BP_ShooterPlayerStart.BP_ShooterPlayerStart_C"))
  (Utilities|Array|Shuffle _outactors)
  (bind _array_element (Utilities|Array|ForEachLoopwithBreak _outactors :!label _label)
    (:LoopBody
      (if (Default|IsFree _array_element)
        (bind _output_get (LocalVariables|SetL_PlayerStart _array_element))
        (bind _newcharacter (Default|SpawnChracter _output_get Player))
        (Utilities|PrintMessage "Spawned Player : " true _newcharacter 15.0)
        (goto _label Break)))))

(fn SpawnSpectator
  (params (Player :type BP%20Shooter%20Controller%20Object%20Reference) (DeathInstigator :type BP%20Shooter%20Controller%20Object%20Reference))
  (LocalVariables|SetL_DeadPlayer Player)
  (bind _output_get (LocalVariables|SetL_DeathInstigator DeathInstigator))
  (Utilities|IsValid _output_get
    (:Is%20Valid
      (LocalVariables|SetL_SpawnTransform (Transformation|GetActorTransform (Pawn|GetControlledPawn (LocalVariables|GetL_DeathInstigator)))))
    (:Is%20Not%20Valid
      (LocalVariables|SetL_SpawnTransform (Transformation|GetActorTransform (Pawn|GetControlledPawn (LocalVariables|GetL_DeadPlayer))))))
  (bind _returnvalue (Game|SpawnActorfromClass (select (Utilities|IsValid (LocalVariables|GetL_DeathInstigator)) "/Game/Blueprints/Player/Spectators/BP_SpectatorFollower.BP_SpectatorFollower_C" "/Game/Blueprints/Player/Spectators/BP_SpectatorFree.BP_SpectatorFree_C") (LocalVariables|GetL_SpawnTransform) "Undefined" 0 (LocalVariables|GetL_DeadPlayer) 0))
  (bind _output_get_2 (LocalVariables|SetL_NewSpectator _returnvalue))
  (bind _asbp_spectator_follower (Utilities|Casting|CastToBP_SpectatorFollower _output_get_2)
    (:then
      (Variables|/Game/Blueprints/Player/Spectators/BP_SpectatorFollower.BP_SpectatorFollower_C|SetPlayerToFollow _asbp_spectator_follower (.AsBP%20Shooter%20Character (Utilities|Casting|CastToBP_ShooterCharacter (Pawn|GetControlledPawn (LocalVariables|GetL_DeathInstigator))))))
    (:CastFailed
      _))
  (Pawn|Possess (LocalVariables|GetL_DeadPlayer) (LocalVariables|GetL_NewSpectator))
  (Utilities|PrintMessage (Utilities|String|Append "Spawned Spectator : " (Utilities|GetDisplayName (LocalVariables|GetL_DeadPlayer)) " For following :  " (Utilities|GetDisplayName (LocalVariables|GetL_DeathInstigator)) " Spektator name is : ") true (LocalVariables|GetL_NewSpectator) 15.0)
  (return (LocalVariables|GetL_NewSpectator)))

(fn LaunchRespawnTimeChecker
  (bind _returnvalue (Utilities|Time|SetTimerbyFunctionName 0 "Respawn" (Variables|Respawn|GetRespawnTime)))
  (Variables|Respawn|SetRespawnTimer _returnvalue))

(fn Start/EndRound
  (params (IsStart :type Boolean) (EndRounReason :type E_RoundFinishReasons%20Enum :default "NewEnumerator0"))
  (LocalVariables|SetL_IsStart IsStart)
  (for _array_element (Variables|/Script/Engine.GameStateBase|GetPlayerArray (Game|GetGameState))
    (bind _asbp_shooter_controller (Utilities|Casting|CastToBP_ShooterController (Components|GetOwner _array_element)))
    (if (LocalVariables|GetL_IsStart)
      (CallFunction|SpawnPlayer _asbp_shooter_controller)
      (else
        (CallFunction|SpawnSpectator _asbp_shooter_controller)
        (Utilities|PrintMessage (Utilities|String|Append "Death :  " (Utilities|String|ToString(Integer) (Variables|/Game/Blueprints/Player/BP_ShooterPlayerState.BP_ShooterPlayerState_C|GetDeath (.AsBP%20Shooter%20Player%20State (Utilities|Casting|CastToBP_ShooterPlayerState (Variables|/Script/Engine.Controller|GetPlayerState _asbp_shooter_controller))))) " For player : ") true _asbp_shooter_controller 15.0))))
  (if (LocalVariables|GetL_IsStart)
    (Default|CallRoundStarted)
    (else
      (Default|CallRoundEnded EndRounReason))))

(fn LaunchTimeChecker
  (Utilities|Time|SetTimerbyFunctionName 0 "CheckTime" 1.0 true))

(fn CheckTime
  (bind _asbp_base_game_state (Utilities|Casting|CastToBP_BaseGameState (Game|GetGameState)))
  (if (>= (Variables|/Game/Blueprints/Game/GameStates/BP_BaseGameState.BP_BaseGameState_C|GetRoundTime _asbp_base_game_state) (Variables|Limits|GetTimeLimit))
    (CallFunction|Start/EndRound false "NewEnumerator0")))