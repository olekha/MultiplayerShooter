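; BP_TeamGameMode is a team-based shooter game mode that adds team rules to its parent's logic.
; On player death it optionally checks the instigator's team points against a limit, then after a short delay ends the round and changes game state.
; Spawning picks a random free BP_ShooterPlayerStart matching the player's team.
; Damage between teammates is blocked unless friendly fire is allowed.
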(event EventBeginPlay
  (|CallParentFunction) ; This node is disabled and will not be called.\nDrag off pins to build functionality.
)

(event EventTick
  (params (DeltaSeconds :type Float%20%28single-precision%29)))

(event EventPlayerDiedEvent
  (params (DeadPlayer :type BP%20Shooter%20Controller%20Object%20Reference) (DeadPlayerCharacter :type BP%20Shooter%20Character%20Object%20Reference) (Instigator :type BP%20Shooter%20Controller%20Object%20Reference) (InstigatorCharacter :type BP%20Shooter%20Character%20Object%20Reference) (DeathCauser :type Actor%20Object%20Reference))
  (|CallParentFunction DeadPlayer DeadPlayerCharacter Instigator InstigatorCharacter DeathCauser)
  (if (Variables|Limits|GetIsLimitByTeamPoints)
    (if (>= (Default|GetTeamPoints (.AsBP%20TM%20in%20Game%20State (Utilities|Casting|CastToBP_TM_InGameState (Game|GetGameState))) (Variables|/Game/Blueprints/Player/BP_TeamPlayerState.BP_TeamPlayerState_C|GetTeam (.AsBP%20Team%20Player%20State (Utilities|Casting|CastToBP_TeamPlayerState (Variables|/Script/Engine.Controller|GetPlayerState Instigator))))) (Variables|Limits|GetTeamPointsLimit))
      (Utilities|FlowControl|Delay 0.2)
      (CallFunction|EndRound "NewEnumerator2" true)
      (CallFunction|ChangeGameState "NewEnumerator2"))))

(fn ConstructionScript
  (|CallParentFunction))

(fn GetFreeSpawnPoint
  (params (Player :type BP%20Shooter%20Controller%20Object%20Reference))
  (bind _outactors (Actor|GetAllActorsOfClass "/Game/Blueprints/Game/BP_ShooterPlayerStart.BP_ShooterPlayerStart_C"))
  (Utilities|Array|Shuffle _outactors)
  (bind _array_element (Utilities|Array|ForEachLoopwithBreak _outactors)
    (:LoopBody
      (if (and (Default|IsFree _array_element) (Utilities|Enum|Equal(Enum) (Variables|/Game/Blueprints/Game/BP_ShooterPlayerStart.BP_ShooterPlayerStart_C|GetTeam _array_element) (Variables|/Game/Blueprints/Player/BP_TeamPlayerState.BP_TeamPlayerState_C|GetTeam (CallFunction|GetControllerTMPlayerState Player))))
        (return _array_element)))))

(fn ShouldDamagePlayer
  (params (Damage :type BP%20Shooter%20Controller%20Object%20Reference) (Instigator :type BP%20Shooter%20Controller%20Object%20Reference))
  (return (or (Utilities|Enum|NotEqual(Enum) (Variables|/Game/Blueprints/Player/BP_TeamPlayerState.BP_TeamPlayerState_C|GetTeam (CallFunction|GetControllerTMPlayerState Damage)) (Variables|/Game/Blueprints/Player/BP_TeamPlayerState.BP_TeamPlayerState_C|GetTeam (CallFunction|GetControllerTMPlayerState Instigator))) (Variables|TeamGameModeSettings|GetAllowFriendlyFire))))