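; Player component that tracks health, armor and stamina for BP_ShooterCharacter, with changes made only on the server.
; It binds to the owner's damage event, records the last instigator and causer, then uses math expressions where armor reduces health loss and wears down.
; Server-side RepNotifies on IsDead and IsTired report deaths with killer details to BP_ShooterPlayerState and signal exhaustion when UseStamina empties stamina.
; Getters expose values and states.
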(event Custom|OnTakeAnyDamage_Event_0
  (params (DamagedActor :type Actor%20Object%20Reference) (Damage :type Float%20%28single-precision%29) (DamageType :type Damage%20Type%20Object%20Reference) (InstigatedBy :type Controller%20Object%20Reference) (DamageCauser :type Actor%20Object%20Reference))
  (if (not (Variables|Health|GetIsDead))
    (Variables|HitInfot|SetLastHitInstigator InstigatedBy)
    (Variables|HitInfot|SetLastHitCausWith DamageCauser)
    (CallFunction|ApplyDamage Damage)))

(event EventBeginPlay
  (bind _asbp_shooter_character (Utilities|Casting|CastToBP_ShooterCharacter (Components|GetOwner)))
  (Variables|Default|SetCharacter _asbp_shooter_character)
  (if (Networking|IsServer)
    (EventDispatchers|AssignOnTakeAnyDamage (Variables|Default|GetCharacter) (EventDispatchers|CreateEvent :!event Custom|OnTakeAnyDamage_Event_0))))

(fn ApplyDamage
  (params (Damage :type Float%20%28single-precision%29))
  (if (Networking|IsServer)
    (LocalVariables|SetL_Damage Damage)
    (Variables|Health|SetHealth (|(clamp(({D118CE90-4EF0-7EDB-618B-A5906273FD14}-({477B13A7-4CD0-3EF0-DAA1-B3B85F862A06}*(1-({E7D3D075-4DE4-CB0A-9945-A4B95FE5D0C0}/200)))),0,{0D8A72CF-498E-7499-E0A0-CFABA19BCAD3}))))
    (Variables|Armor|SetArmor (|(clamp(({E7D3D075-4DE4-CB0A-9945-A4B95FE5D0C0}-({477B13A7-4CD0-3EF0-DAA1-B3B85F862A06}*{FDF92909-4A35-2FEA-86CE-A79AF765DB4C})),0,{D2DD9E53-4819-9AD5-1324-4293BEBAAA53}))))
    (if (<= (Variables|Health|GetHealth) 0.0)
      (Variables|Health|SetIsDead true)
      (else
        (Variables|Health|SetIsDead false)))))

(fn UseStamina
  (params (How%20Much :type Float%20%28single-precision%29))
  (if (Networking|IsServer)
    (bind _output_get (Variables|Stamina|SetStamina (Math|Float|Clamp(Float) (- (Variables|Stamina|GetStamina) How%20Much) 0.0 (Variables|Stamina|GetMaxStamina))))
    (if (<= _output_get 0.0)
      (Variables|Stamina|SetIsTired true)
      (else
        (Variables|Stamina|SetIsTired false)))))

(fn OnRepIsTired
  (if (Networking|IsServer)
    (if (Variables|Stamina|GetIsTired)
      (Default|CallCharacterTired)
      (Development|PrintString "Character Tired"))))

(fn OnRepIsDead
  (bind _character (Variables|Default|GetCharacter))
  (bind _lasthitinstigator (Variables|HitInfot|GetLastHitInstigator))
  (if (Networking|IsServer)
    (if (Variables|Health|GetIsDead)
      (bind _asbp_shooter_player_state (Utilities|Casting|CastToBP_ShooterPlayerState (Variables|/Script/Engine.Pawn|GetPlayerState (Variables|Default|GetCharacter))))
      (Default|PlayerDied _asbp_shooter_player_state (.AsBP%20Shooter%20Controller (Utilities|Casting|CastToBP_ShooterController (Pawn|GetController _character))) _character (.AsBP%20Shooter%20Controller (Utilities|Casting|CastToBP_ShooterController _lasthitinstigator)) (.AsBP%20Shooter%20Character (Utilities|Casting|CastToBP_ShooterCharacter (Pawn|GetControlledPawn _lasthitinstigator))) (Variables|HitInfot|GetLastHitCausWith)))))

(fn GetHealth
  (return (Variables|Health|GetHealth) (Variables|Health|GetMaxHealth)))

(fn GetArmor
  (return (Variables|Armor|GetArmor) (Variables|Armor|GetMaxArmor)))

(fn GetStamina
  (return (Variables|Stamina|GetStamina) (Variables|Stamina|GetMaxStamina)))

(fn CheckIsDead
  (return (Variables|Health|GetIsDead)))

(fn CheckIsTired
  (return (Variables|Stamina|GetIsTired)))