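; BPC_WeaponsManager is a player component that creates and tracks the shooter character's main, secondary and grenade weapons.
; BeginPlay casts the owner to BP_ShooterCharacter and caches it as the character.
; CreateWeapon runs only on the server, spawning a weapon owned by the character's controller, storing it by weapon type and attaching it to the character.
; AddWeapon is an empty stub, and nothing here calls CreateWeapon.
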(event EventBeginPlay
  (Utilities|FlowControl|Sequence
    (:then_0
      (|InitialVariablesSetup))))

(event EventTick
  (params (DeltaSeconds :type Float%20%28single-precision%29)))

(fn CreateWeapon
  (params (Class :type BP%20Weapon%20Class%20Reference))
  (bind _character (Variables|Default|GetCharacter))
  (if (Networking|IsServer)
    (bind _returnvalue (Game|SpawnActorfromClass Class (Math|Transform|MakeTransform "0, 0, 0" "0, 0, 0" "1,1,1") "AlwaysSpawn" (Pawn|GetController _character) _character))
    (LocalVariables|SetL_Weapon _returnvalue)
    (Utilities|FlowControl|Sequence
      (:then_0
        (switch Utilities|FlowControl|Switch|SwitchonE_WeaponType (Variables|/Game/Blueprints/Weapons/BP_Weapon.BP_Weapon_C|GetWeaponType (LocalVariables|GetL_Weapon))
          (:NewEnumerator0
            (Variables|Default|SetMainWeapon (LocalVariables|GetL_Weapon)))
          (:NewEnumerator1
            (Variables|Default|SetSecondaryWeapon (LocalVariables|GetL_Weapon)))
          (:NewEnumerator2
            (Variables|Default|SetGrenades (LocalVariables|GetL_Weapon)))))
      (:then_1
        (Transformation|AttachActorToActor (LocalVariables|GetL_Weapon) (Variables|Default|GetCharacter) "None" "SnapToTarget" "SnapToTarget" "KeepRelative" true)))))

(fn AddWeapon)