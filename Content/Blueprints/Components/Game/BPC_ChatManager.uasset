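; BPC_ChatManager is a chat component that relays player messages and toggles each player's chat.
; SendMessage passes the player and message to AllMessagesSent, which fires the MessageSent dispatcher for listeners.
; ActivateChat validates the chat reference on the player's HUD, then calls ActivateChatOnClient to set its active state.
; CheckIsChatActivated reads the active flag from that same reference, without a validity check.
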(event Custom|AllMessagesSent
  (params (Plyer :type BP%20Shooter%20Player%20State%20Object%20Reference) (Message :type Text))
  (Default|CallMessageSent Plyer Message))

(event Custom|ActivateChatOnClient
  (params (activate :type Boolean) (Player :type BP%20Shooter%20Controller%20Object%20Reference))
  (Default|ActivateChat (Variables|/Game/Blueprints/Game/BP_ShooterHUD.BP_ShooterHUD_C|GetChatReference (CallFunction|GetControllerSHUD Player)) activate))

(fn SendMessage
  (params (Player :type BP%20Shooter%20Player%20State%20Object%20Reference) (Message :type Text))
  (CallFunction|AllMessagesSent Player Message))

(fn CheckIsChatActivated
  (params (Player :type BP%20Shooter%20Controller%20Object%20Reference))
  (return (Variables|/Game/UI/Chat/WD_Chat.WD_Chat_C|GetIsChatActive (Variables|/Game/Blueprints/Game/BP_ShooterHUD.BP_ShooterHUD_C|GetChatReference (CallFunction|GetControllerSHUD Player)))))

(fn ActivateChat
  (params (Activate :type Boolean) (Player :type BP%20Shooter%20Controller%20Object%20Reference))
  (Utilities|IsValid (Variables|/Game/Blueprints/Game/BP_ShooterHUD.BP_ShooterHUD_C|GetChatReference (CallFunction|GetControllerSHUD Player))
    (:Is%20Valid
      (CallFunction|ActivateChatonClient Activate Player))))