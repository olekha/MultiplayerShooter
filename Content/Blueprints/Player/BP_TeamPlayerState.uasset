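; BP_TeamPlayerState is a player state that adds a team to the parent's spectator handling.
; Outside of play, spectating is represented as a team value: SetTeam updates the spectator flag, and SetIsSpectator moves spectators to that team.
; CheckIsSpectator defers to the parent for in-game queries and otherwise compares the team to the spectator value.
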(event EventSetIsSpectator
  (params (IsSpectator :type Boolean) (IsInGame :type Boolean))
  (|CallParentFunction IsSpectator IsInGame)
  (if (and IsSpectator (not IsInGame))
    (Variables|Default|SetTeam "NewEnumerator3")))

(fn ConstructionScript
  (|CallParentFunction))

(fn SetTeam
  (params (NewTeam :type E_Teams%20Enum :default "NewEnumerator0"))
  (bind _output_get (Variables|Default|SetTeam NewTeam))
  (CallFunction|SetIsSpectator (Utilities|Enum|Equal(Enum) _output_get "NewEnumerator3") false))

(fn GetPlayerTeam
  (return (Variables|Default|GetTeam)))

(fn CheckIsSpectator
  (params (InGame :type Boolean))
  (return (select InGame (|CallParentFunction true) (Utilities|Enum|Equal(Enum) (Variables|Default|GetTeam) "NewEnumerator3"))))