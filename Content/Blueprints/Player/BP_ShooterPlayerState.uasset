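; Shooter player state that tracks a player's alive and in-game or out-of-game spectator status and handles timed respawns.
; On the server, it binds to game state round-end and spawn events once in-game, updating flags for its own controller.
; Deaths are multicast, clearing the alive flag on authority and relaying to the game state.
; The respawn timer calls the game mode's SpawnPlayer and is paused on round end or character spawn.
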(event Custom|ChangedGameState_Event_0
  (params (NewGameState :type E_GameStateTypes%20Enum :default "NewEnumerator0"))
  (bind _gs (CallFunction|GetSGameState))
  ;[1 1 1] Changed Game State
  (switch Utilities|FlowControl|Switch|SwitchonE_GameStateTypes NewGameState
    (:NewEnumerator1
      (EventDispatchers|AssignRoundEnded _gs (delegate Custom|RoundEnded_Event_0))
      (EventDispatchers|AssignCharacterSpawned _gs (EventDispatchers|CreateEvent :!event Custom|CharacterSpawned_Event))
      (EventDispatchers|AssignSpectatorSpawned _gs (EventDispatchers|CreateEvent :!event Custom|SpectatorSpawned_Event_0)))))

(event Custom|RoundEnded_Event_0
  (params (EndingReason :type E_RoundFinishReasons%20Enum :default "NewEnumerator0"))
  ;[1 1 1] Changed Game State
  (CallFunction|StopRespawnTimer))

(event Custom|SpectatorSpawned_Event_0
  (params (Spectator :type BP%20Spectator%20Object%20Reference) (Player :type BP%20Shooter%20Controller%20Object%20Reference) (LookAtCharacter :type BP%20Shooter%20Character%20Object%20Reference))
  (if (== Player (CallFunction|GetPlayerStateOwnerasSController self))
    (Utilities|Casting|CastToBP_SpectatorFollower Spectator
      (:then
        (CallFunction|SetIsSpectator true true))
      (:CastFailed
        (CallFunction|SetIsSpectator true false)))))

(event Custom|PlayerDied
  (params (DeadPlayer :type BP%20Shooter%20Controller%20Object%20Reference) (DeadPlayerCharacter :type BP%20Shooter%20Character%20Object%20Reference) (Instigator :type BP%20Shooter%20Controller%20Object%20Reference) (InstigatorCharacter :type BP%20Shooter%20Character%20Object%20Reference) (KilldWith :type Actor%20Object%20Reference))
  ;[1 1 1] Player Died Multicast
  (CallFunction|PlayerDiedMulticast DeadPlayer DeadPlayerCharacter Instigator InstigatorCharacter KilldWith))

(event Custom|CharacterSpawned_Event
  (params (Player :type BP%20Shooter%20Controller%20Object%20Reference) (Character :type BP%20Shooter%20Character%20Object%20Reference))
  (if (== Player (CallFunction|GetPlayerStateOwnerasSController self))
    (Variables|Default|SetIsAlive true)
    (Variables|Default|SetPlayerCharacter Character)
    (CallFunction|SetIsSpectator false true)
    (CallFunction|SetIsSpectator false false)
    (CallFunction|StopRespawnTimer)))

(event Custom|PlayerDied_Multicast
  (params (DeadPlayer :type BP%20Shooter%20Controller%20Object%20Reference) (DeadPlayerCharacter :type BP%20Shooter%20Character%20Object%20Reference) (Instigator :type BP%20Shooter%20Controller%20Object%20Reference) (InstigatorCharacter :type BP%20Shooter%20Character%20Object%20Reference) (DeathCauser :type Actor%20Object%20Reference))
  ;[1 1 1] Player Died Multicast
  (Networking|SwitchHasAuthority
    (:Authority
      (Variables|Default|SetIsAlive false))
    (:Remote
      _))
  (Default|CallPlayerDied (CallFunction|GetSGameState) DeadPlayer DeadPlayerCharacter Instigator InstigatorCharacter DeathCauser))

(event EventBeginPlay
  (Variables|Default|SetPlayerController (CallFunction|GetPlayerStateOwnerasSController self))
  (Networking|SwitchHasAuthority
    (:Authority
      (EventDispatchers|AssignChangedGameState (CallFunction|GetSGameMode) (EventDispatchers|CreateEvent :!event Custom|ChangedGameState_Event_0)))))

(fn ConstructionScript)

(fn LaunchRespawnTimer
  (params (Time :type Float%20%28single-precision%29))
  (bind _returnvalue (Utilities|Time|SetTimerbyFunctionName 0 "Respawn" (+ Time (Variables|Spawn|GetSpawnTimeFault))))
  (Variables|Spawn|SetRespawnTimer _returnvalue))

(fn Respawn
  (bind _asbp_shooter_game_mode (Utilities|Casting|CastToBP_ShooterGameMode (Game|GetGameMode)))
  (Default|SpawnPlayer _asbp_shooter_game_mode (Variables|Default|GetPlayerController)))

(fn CheckIsAlive
  (return (Variables|Default|GetIsAlive)))

(fn CheckIsSpectator
  (params (InGame :type Boolean))
  (return (select InGame (Variables|Default|GetIsInGameSpectator) (Variables|Default|GetIsOutOfGameSpectator))))

(fn SetIsSpectator
  (params (IsSpectator :type Boolean) (IsInGame :type Boolean))
  (if IsInGame
    (Variables|Default|SetIsInGameSpectator IsSpectator)
    (else
      (Variables|Default|SetIsOutOfGameSpectator IsSpectator))))

(fn StopRespawnTimer
  (Utilities|Time|PauseTimerbyHandle (Variables|Spawn|GetRespawnTimer)))