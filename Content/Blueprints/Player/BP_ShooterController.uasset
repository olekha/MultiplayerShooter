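; Player controller for the shooter that handles player requests and drives HUD widgets through match phases, death, spawning and spectating.
; Server events forward team changes, spectator switches, respawns and chat messages to game mode, game state or player state.
; On authority it binds game mode and state dispatchers, relaying them to client events that initialize or toggle widgets.
; Tab held shows the tab menu; Enter fast-respawns spectators when allowed, otherwise opens chat for non-spectators.
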(event Custom|ServerRespawn
  ;[1 1 1] Buttons Event
  ;;[0 0.2215 1] Respawn
  (Default|SpawnPlayer (CallFunction|GetSGameMode) self))

(event Custom|ServerRequestChangeTeam
  (params (NewTeam :type E_Teams%20Enum :default "NewEnumerator0") (IsInGame :type Boolean))
  (bind _gs (CallFunction|GetTMGameState))
  (bind _self self)
  (bind _splayerstate (CallFunction|GetControllerTMPlayerState _self))
  (Utilities|IsValid _gs
    (:Is%20Valid
      (if IsInGame
        (Default|ChangePlayerTeam _gs _splayerstate NewTeam)
        (else
          (Default|SetTeam _splayerstate NewTeam))))))

(event Custom|ServerRequestBecomeChar/Spect
  (params (IsSpectator :type Boolean) (IsInGame :type Boolean))
  (bind _gs (CallFunction|GetDMGameState))
  (bind _self self)
  (bind _splayerstate (CallFunction|GetControllerSPlayerState _self))
  (Utilities|IsValid _gs
    (:Is%20Valid
      (if IsInGame
        (Default|BecamePlayer _gs IsSpectator _splayerstate)
        (else
          (Default|SetIsSpectator _splayerstate IsSpectator false))))))

(event Input|KeyboardEvents|Tab
  (params (Key :type Key%20Structure))
  (bind _gs (CallFunction|GetSGameState))
  (bind _self self)
  (bind _self_2 self)
  (bind _isinplay (Default|CheckIsinPlay _gs))
  (bind _s_hud (CallFunction|GetControllerSHUD _self_2))
  (bind _splayerstate (CallFunction|GetControllerSPlayerState _self))
  (bind _isspectator (Default|CheckIsSpectator _splayerstate false))
  (bind _returnvalue (not _isspectator))
  (bind _returnvalue_2 (and _isinplay _returnvalue))
  ;[1 1 1] Buttons Event
  ;;[0 0.2215 1] Show Hide Tab Menu
  (:Pressed
    (if _returnvalue_2
      (Default|ToggleWidgets _s_hud false true false false false false false)))
  (:Released
    (if _returnvalue_2
      (Default|ToggleWidgets _s_hud true false (== (Utilities|GetClass (Pawn|GetControlledPawn)) "/Game/Blueprints/Player/Spectators/BP_Spectator.BP_Spectator_C") false false false false))))

(event Input|KeyboardEvents|Enter
  (params (Key :type Key%20Structure))
  ;[1 1 1] Buttons Event
  ;;[0 0.2215 1] Respawn
  (:Pressed
    (if (Default|CheckIsSpectator (.AsBP%20Shooter%20Player%20State (Utilities|Casting|CastToBP_ShooterPlayerState (Variables|GetPlayerState))) true)
      (Utilities|Casting|CastToBP_Spectator (Pawn|GetControlledPawn))
      (if (Variables|/Game/Blueprints/Game/BP_ShooterGameMode.BP_ShooterGameMode_C|GetIsAllowFastRespawn (CallFunction|GetSGameMode))
        (CallFunction|ServerRespawn)))))

(event Custom|FreeSpectSpawn_OwningClient
  ;[1 1 1] ShowSpectatorHUDorPlayerStats
  (Default|ToggleWidgets (CallFunction|GetControllerSHUD self) false false false false false true true))

(event Custom|InitPostGameWidgetsOnClient
  (Default|InitPostRoundMenu (CallFunction|GetControllerSHUD self)))

(event Custom|PlayerDied_OwningClient
  ;[1 1 1] HideHUDAfterDeath
  (Default|ToggleHUD (CallFunction|GetControllerSHUD self) false))

(event Custom|FolowerSpectSpawn_OwningClient
  ;[1 1 1] ShowSpectatorHUDorPlayerStats
  (Default|ToggleWidgets (CallFunction|GetControllerSHUD self) false false true false false false true))

(event Custom|InitPreGameWidgetsOnClient
  (bind _self self)
  (bind _s_hud (CallFunction|GetControllerSHUD _self))
  (Default|InitPreRoubdMenu _s_hud)
  (Default|InitChat _s_hud))

(event Custom|PostMessageInChatOnServer
  (params (Message :type Text))
  (Default|SendMessage (Variables|/Game/Blueprints/Game/GameStates/BP_ShooterGameState.BP_ShooterGameState_C|GetBPC_Chat (CallFunction|GetSGameState)) (CallFunction|GetControllerSPlayerState self) Message))

(event Custom|CharacterSpawned_Event
  (params (Player :type BP%20Shooter%20Controller%20Object%20Reference) (Character :type BP%20Shooter%20Character%20Object%20Reference))
  ;[1 1 1] ShowHUDAfterSpawn
  (if (== Player self)
    (CallFunction|CharacterSpawnedOwningClient)))

(event Custom|PlayerDied_Event
  (params (DeadPlayer :type BP%20Shooter%20Controller%20Object%20Reference) (DeadPlayerCharacter :type BP%20Shooter%20Character%20Object%20Reference) (Instigator :type BP%20Shooter%20Controller%20Object%20Reference) (InstigatorCharacter :type BP%20Shooter%20Character%20Object%20Reference) (DeathCauser :type Actor%20Object%20Reference))
  ;[1 1 1] HideHUDAfterDeath
  (if (== DeadPlayer self)
    (CallFunction|PlayerDiedOwningClient)))

(event Custom|SpectatorSpawned_Event
  (params (Spectator :type BP%20Spectator%20Object%20Reference) (Player :type BP%20Shooter%20Controller%20Object%20Reference) (LookAtCharacter :type BP%20Shooter%20Character%20Object%20Reference))
  ;[1 1 1] ShowSpectatorHUDorPlayerStats
  (if (== Player self)
    (Utilities|Casting|CastToBP_SpectatorFollower Spectator
      (:then
        (CallFunction|FolowerSpectSpawnOwningClient))
      (:CastFailed
        (CallFunction|FreeSpectSpawnOwningClient)))))

(event Custom|CharacterSpawned_OwningClient
  ;[1 1 1] ShowHUDAfterSpawn
  (Default|ToggleWidgets (CallFunction|GetControllerSHUD self) true false false false false false true))

(event Custom|InitInGameWidgetsOnClient
  (bind _self self)
  (bind _s_hud (CallFunction|GetControllerSHUD _self))
  (Default|InitHUD _s_hud)
  (Default|InitFolowerSpectMenu _s_hud)
  (Default|InitFreeSpectMenu _s_hud)
  (Default|InitTabMenu _s_hud))

(event Custom|ChangedGameState_Event_0
  (params (NewGameState :type E_GameStateTypes%20Enum :default "NewEnumerator0"))
  (switch Utilities|FlowControl|Switch|SwitchonE_GameStateTypes NewGameState
    (:NewEnumerator0
      (CallFunction|InitPreGameWidgetsonClient)
      (CallFunction|ToggleWidgetsonClient false false false true false false true))
    (:NewEnumerator1
      (CallFunction|InitinGameWidgetsonClient)
      (CallFunction|ToggleWidgetsonClient true false false false false false true))
    (:NewEnumerator2
      (CallFunction|InitPostGameWidgetsonClient)
      (CallFunction|ToggleWidgetsonClient false false false false true false true))))

(event Custom|ToggleWidgetsOnClient
  (params (ShowHUD :type Boolean) (ShowTabMenu :type Boolean) (ShowFolowerSpectMenu :type Boolean) (ShowPreRoundMenu :type Boolean) (ShowPostRoundMenu :type Boolean) (ShowFreeSpectMenu :type Boolean) (ShowChat :type Boolean))
  (Default|ToggleWidgets (CallFunction|GetControllerSHUD self) ShowHUD ShowTabMenu ShowFolowerSpectMenu ShowPreRoundMenu ShowPostRoundMenu ShowFreeSpectMenu ShowChat))

(event EventBeginPlay
  (bind _gs (CallFunction|GetSGameState))
  (Networking|SwitchHasAuthority
    (:Authority
      (EventDispatchers|AssignChangedGameState (CallFunction|GetSGameMode) (EventDispatchers|CreateEvent :!event Custom|ChangedGameState_Event_0))
      (EventDispatchers|AssignCharacterSpawned _gs (EventDispatchers|CreateEvent :!event Custom|CharacterSpawned_Event))
      (EventDispatchers|AssignPlayerDied _gs (EventDispatchers|CreateEvent :!event Custom|PlayerDied_Event))
      (EventDispatchers|AssignSpectatorSpawned _gs (EventDispatchers|CreateEvent :!event Custom|SpectatorSpawned_Event)))))

(event Input|KeyboardEvents|Enter
  (params (Key :type Key%20Structure))
  (bind _gs (CallFunction|GetSGameState))
  (bind _bpc_chat (Variables|/Game/Blueprints/Game/GameStates/BP_ShooterGameState.BP_ShooterGameState_C|GetBPC_Chat _gs))
  (:Pressed
    (if (not (Default|CheckIsSpectator (.AsBP%20Shooter%20Player%20State (Utilities|Casting|CastToBP_ShooterPlayerState (Variables|GetPlayerState))) true))
      (if (not (Components|Activation|IsActive _bpc_chat))
        (Default|ActivateChat _bpc_chat true self)))))

(fn ConstructionScript)